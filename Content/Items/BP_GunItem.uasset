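; Gun item that the player uses with a "Shoot" action to fire a hitscan shot.
; UseObject line-traces along the use direction, playing a gunshot, spawning a muzzle flash and randomly sized bullet-hole decal, and applying point damage to any hit actor.
; If the player's highlighted actor is a ThemeHolder, it defers to the parent's use behavior instead of firing.
; Its Interact override always returns false.
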(event Custom|StopInteract
  (params (ActorStopingInteract :type Actor%20Object%20Reference))
  (|CallParentFunction ActorStopingInteract))

(event EventBeginPlay
  (Collision|SetCollisionResponsetoChannel (Variables|Default|GetItemStaticMesh) "ECC_GameTraceChannel1" "ECR_Ignore"))

(event Collision|EventActorBeginOverlap
  (params (OtherActor :type Actor%20Object%20Reference)))

(event EventTick
  (params (DeltaSeconds :type Float%20%28single-precision%29)))

(event EventUseObject
  (params (UseDirection :type Vector :default "0, 0, 0") (UsePosition :type Vector :default "0, 0, 0") (ActorUsingObject :type Actor%20Object%20Reference))
  (bind _returnvalue (Class|PlayerCharacter|GetCurrentlyHighlightedActor (Variables|Default|GetPlayerCharacter)))
  (Utilities|Casting|CastToThemeHolder _returnvalue
    (:then
      (|CallParentFunction UseDirection UsePosition ActorUsingObject))
    (:CastFailed
      (Audio|PlaySound2D "/Game/Items/Meshes/FPS_Guns_4K_-_Pistol_2/gun-shot-359196.gun-shot-359196" 1.0 1.0 0.0 0 0)
      (bind _outhit (Collision|LineTraceByChannel UsePosition (+ UsePosition (* UseDirection 1e+04)) "TraceTypeQuery1" false (Utilities|Array|MakeArray (Variables|Default|GetPlayerCharacter)) "None"))
      (Rendering|Decal|SpawnDecalatLocation "/Game/Items/Meshes/FPS_Guns_4K_-_Pistol_2/M_BulletHole.M_BulletHole" (Math|Conversions|ToVector(Float) (Math|Random|RandomIntegerinRange 3 7)) (.location _outhit) (Math|Conversions|RotationFromXVector (.impactnormal _outhit)) 2e+01)
      (Niagara|SpawnSystemAttached "/Game/MuzzleFlash/MuzzleFlash/Niagara/NS_MuzzleFlash.NS_MuzzleFlash" (Variables|Default|GetItemStaticMesh) "MuzzleFlash" "0, 0, 0" "0, 0, 0" "KeepRelativeOffset" true)
      (Utilities|IsValid (.hitactor _outhit)
        (:Is%20Valid
          (Game|Damage|ApplyPointDamage (.hitactor _outhit) 1e+01 UseDirection (Collision|MakeHitResult false false 0.0 0.0 "0, 0, 0" "0, 0, 0" "0,0,1" "0,0,1" 0 0 0 (.hitbonename _outhit) "None" 0 0 0 "0, 0, 0" "0, 0, 0")))))))

(fn ConstructionScript)

(fn GetUseActionName
  (return "Shoot"))

(fn Interact
  (params (ActorThatInteract :type Actor%20Object%20Reference))
  (return false))