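; Interactable Word Scrambler machine that takes two ItemTheme items and yields a scrambled item for the player to retrieve.
; Interact runs a state machine for opening, loading via the holder socket, closing and retrieval.
; The second item triggers ScrambleItems, electric effects, sound and timeline shake, until the glass widget's animation-finished event reopens it.
; The widget's render target feeds the screen material, and an overlay material highlights laser hits.
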(event Custom|Scramblerstarts
  (bind _returnvalue (Math|Random|RandomFloatinRange -2.0 2.0))
  (bind (_output _output2) (Utilities|UpdateGlassUI))
  (bind _returnvalue_2 (Class|WordScrambler|ScrambleItems _output _output2))
  (bind _output_get (Variables|Default|SetScrambledItem _returnvalue_2))
  (Class|Item|SetupItemAttachment _output_get)
  (Transformation|AttachComponentToComponent _output_get (Variables|Default|GetSkeletalMesh) "HolderSocket" "SnapToTarget" "KeepWorld" "KeepWorld" true)
  (Utilities|FlowControl|Delay 1.0)
  (Components|Activation|Activate (Variables|Default|GetNS_Electric) false)
  (CallFunction|PlayScramblerSound true)
  (Timeline|Timeline PlayFromStart
    (:Update
      (Transformation|SetRelativeLocation (Variables|Default|GetSkeletalMesh) (Math|Vector|MakeVector _returnvalue _returnvalue _returnvalue) false false))
    (:Finished
      (Transformation|SetRelativeLocation (Variables|Default|GetSkeletalMesh) (Math|Vector|MakeVector 0.0 0.0 0.0) false false))))

(event Custom|ScramblingAnimationFinished
  (Components|Activation|Activate (Variables|Default|GetNiagara) true)
  (Components|Activation|Deactivate (Variables|Default|GetNS_Electric))
  (CallFunction|PlayScramblerSound false)
  (Components|Timeline|SetNewTime (Variables|Default|GetTimeline) 1e+01)
  (Animation|Montage|PlayMontage (Variables|Default|GetSkeletalMesh) "/Game/WordScrambler/Mesh/OpeningStatic_001_Montage.OpeningStatic_001_Montage"
    (:OnCompleted
      (Collision|SetCollisionResponsetoChannel (Variables|Default|GetSkeletalMesh) "ECC_GameTraceChannel1" "ECR_Block")
      (Variables|Default|SetCurrentState "FinishedProcessing"))))

(event EventBeginPlay
  (bind _skeletalmesh (Variables|Default|GetSkeletalMesh))
  (bind _returnvalue (Rendering|Material|CreateDynamicMaterialInstance "/Game/FXMaterials/OverlayFx/M_DestroyableObjectOverlayMat.M_DestroyableObjectOverlayMat" "None" "None" :!class /Script/Engine.KismetMaterialLibrary))
  (Rendering|Material|SetOverlayMaterial _skeletalmesh _returnvalue :!class /Script/Engine.MeshComponent)
  (bind _returnvalue_2 (Rendering|Material|CreateDynamicMaterialInstance _skeletalmesh 1 "/Game/WordScrambler/Mesh/glass.glass" "None" :!class /Script/Engine.PrimitiveComponent))
  (Variables|Default|SetScreenDynamicMaterial _returnvalue_2)
  (EventDispatchers|BindEventtoOnScrambleStart (delegate Custom|Scramblerstarts))
  (bind _asuw_item_scrambler_glass (Utilities|Casting|CastToUW_ItemScramblerGlass (UserInterface|GetWidget (Variables|Default|GetWidget))))
  (EventDispatchers|BindEventtoScramblinganimationfinished _asuw_item_scrambler_glass (delegate Custom|ScramblingAnimationFinished)))

(event Collision|EventActorBeginOverlap
  (params (OtherActor :type Actor%20Object%20Reference)))

(event EventTick
  (params (DeltaSeconds :type Float%20%28single-precision%29))
  (bind _widget (Variables|Default|GetWidget))
  (bind _returnvalue (Class|WidgetComponent|GetRenderTarget _widget))
  (if (not (Variables|Default|GetTextureWasSet))
    (Utilities|IsValid _returnvalue
      (:Is%20Valid
        (Rendering|Material|SetTextureParameterValue (Variables|Default|GetScreenDynamicMaterial) "EmissiveTexture" _returnvalue)))))

(event EventOnHitbyPlayerLaser
  (bind _asmaterial_instance_dynamic (Utilities|Casting|CastToMaterialInstanceDynamic (Rendering|Material|GetOverlayMaterial (Variables|Default|GetSkeletalMesh) :!class /Script/Engine.MeshComponent)))
  (Rendering|Material|SetScalarParameterValue _asmaterial_instance_dynamic "HighlightStrenght" 1.0 :!class /Script/Engine.MaterialInstanceDynamic))

(event EventOnNoLongerHitbyPlayerLaser
  (bind _asmaterial_instance_dynamic (Utilities|Casting|CastToMaterialInstanceDynamic (Rendering|Material|GetOverlayMaterial (Variables|Default|GetSkeletalMesh) :!class /Script/Engine.MeshComponent)))
  (Rendering|Material|SetScalarParameterValue _asmaterial_instance_dynamic "HighlightStrenght" 0.0 :!class /Script/Engine.MaterialInstanceDynamic))

(fn ConstructionScript)

(fn Interact
  (params (ActorThatInteract :type Actor%20Object%20Reference))
  (bind _skeletalmesh (Variables|Default|GetSkeletalMesh))
  (bind _skeletalmesh_2 (Variables|Default|GetSkeletalMesh))
  (bind _scrambleditem (Variables|Default|GetScrambledItem))
  (bind _skeletalmesh_3 (Variables|Default|GetSkeletalMesh))
  (bind _attacheditemthemes (Variables|Default|GetAttacheditemThemes))
  (switch Utilities|FlowControl|Switch|SwitchonEWordScramblerState (Variables|Default|GetCurrentState)
    (:Closed
      (Components|Animation|PlayAnimation (Variables|Default|GetSkeletalMesh) "/Game/WordScrambler/Mesh/OpeningStatic_001.OpeningStatic_001" false)
      (Audio|PlaySound2D "/Game/WordScrambler/kamranbashirb-car-door-open-297265.kamranbashirb-car-door-open-297265" 1.0 1.0 0.0 0 0)
      (Variables|Default|SetCurrentState "Opened")
      (Variables|Default|SetShouldDropInteractionWithCurrentObject true)
      (return false))
    (:Opened
      (bind _asplayer_character (Utilities|Casting|CastToPlayerCharacter ActorThatInteract)
        (:then
          (if (== (Utilities|Set|Length (Variables|Default|GetAttacheditemThemes)) 0)
            (Components|Animation|PlayAnimation _skeletalmesh_3 "/Game/WordScrambler/Mesh/ClosingStatic.ClosingStatic" false)
            (Components|Animation|SetPosition _skeletalmesh_3 1.0 true)
            (Audio|PlaySound2D "/Game/WordScrambler/kamranbashirb-car-door-open-297265.kamranbashirb-car-door-open-297265" 1.0 1.0 0.0 0 0)
            (Variables|Default|SetCurrentState "Closed")
            (Variables|Default|SetShouldDropInteractionWithCurrentObject false)
            (return false)
            (else
              (bind _result (Utilities|Set|ToArray _attacheditemthemes))
              (Class|ThemeHolder|DetachfromHolder (Utilities|Array|Get(acopy) _result (Utilities|Array|LastIndex _result)))
              (Class|PlayerCharacter|InteractwithActor _asplayer_character (Utilities|Array|Get(acopy) _result (Utilities|Array|LastIndex _result)))
              (Utilities|Array|RemoveItem _result (Utilities|Array|Get(acopy) _result (Utilities|Array|LastIndex _result)))
              (Utilities|Set|Clear _attacheditemthemes))))
        (:CastFailed
          (bind _asitem_theme (Utilities|Casting|CastToItemTheme ActorThatInteract))
          (Class|Item|SetupItemAttachment _asitem_theme)
          (Transformation|AttachComponentToComponent _asitem_theme (Variables|Default|GetSkeletalMesh) "HolderSocket" "SnapToTarget" "KeepWorld" "KeepWorld" true)
          (Utilities|Set|Add (Variables|Default|GetAttacheditemThemes) _asitem_theme)
          (if (== (Utilities|Set|Length (Variables|Default|GetAttacheditemThemes)) 2)
            (Variables|Default|SetCurrentState "Filled")
            (Components|Animation|PlayAnimation _skeletalmesh "/Game/WordScrambler/Mesh/ClosingStatic.ClosingStatic" false)
            (Components|Animation|SetPosition _skeletalmesh 1.0 true)
            (Audio|PlaySound2D "/Game/WordScrambler/kamranbashirb-car-door-open-297265.kamranbashirb-car-door-open-297265" 1.0 1.0 0.0 0 0)
            (Default|CallOnScrambleStart)
            (Collision|SetCollisionResponsetoChannel (Variables|Default|GetSkeletalMesh) "ECC_GameTraceChannel1" "ECR_Ignore")))))
    (:FinishedProcessing
      (bind _asplayer_character_2 (Utilities|Casting|CastToPlayerCharacter ActorThatInteract))
      (Class|ThemeHolder|DetachfromHolder _scrambleditem)
      (Class|PlayerCharacter|InteractwithActor _asplayer_character_2 _scrambleditem)
      (Components|Animation|PlayAnimation _skeletalmesh_2 "/Game/WordScrambler/Mesh/ClosingStatic.ClosingStatic" false)
      (Components|Animation|SetPosition _skeletalmesh_2 1.0 true)
      (Audio|PlaySound2D "/Game/WordScrambler/kamranbashirb-car-door-open-297265.kamranbashirb-car-door-open-297265" 1.0 1.0 0.0 0 0)
      (Variables|Default|SetCurrentState "Closed")
      (Variables|Default|SetShouldDropInteractionWithCurrentObject false)
      (Utilities|Set|Clear (Variables|Default|GetAttacheditemThemes))
      (return false))))

(fn GetInteractionActionName
  (switch Utilities|FlowControl|Switch|SwitchonEWordScramblerState (Variables|Default|GetCurrentState)
    (:Closed
      (return "Open"))
    (:Opened
      (return "Place Item"))
    (:Filled
      _)
    (:Processing
      _)
    (:FinishedProcessing
      (return "Retrieve item")))
  (return ""))

(fn PlayScramblerSound
  (params (ongoing :type Boolean))
  (bind _washingmachinesoundcue (Variables|Default|GetWashingMachinesoundcue))
  (Effects|Components|ParticleSystem|SetBoolParameter _washingmachinesoundcue "Ongoing" ongoing)
  (Audio|Components|Audio|Play _washingmachinesoundcue 0.0)
  (if (not ongoing)
    (Audio|Components|Audio|FadeOut _washingmachinesoundcue 4.0 0.0 "Logarithmic" :!class /Script/Engine.AudioComponent)))