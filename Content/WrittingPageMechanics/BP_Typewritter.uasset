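; Interactable typewriter that lets the player start and quit typing on a child BP_BasePaper.
; Interact switches input to the paper's widget, then hands Myles to a spawned AI controller given the standing position as destination.
; StopInteract restores game input and movement, clears sitting/typing animations and stops paper writing.
; A dynamic overlay material highlights the mesh while the player's laser hits it.
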(event EventBeginPlay
  (Utilities|FlowControl|Delay 0.1)
  (ChildActorComponent|SetChildActorClass (Variables|Default|GetChildActor) "/Game/WrittingPageMechanics/BP_BasePaper.BP_BasePaper_C")
  (Variables|Default|SetChildActorRelativeTransform (Transformation|GetRelativeTransform (Variables|Default|GetChildActor)))
  (bind _returnvalue (Rendering|Material|CreateDynamicMaterialInstance "/Game/FXMaterials/OverlayFx/M_DestroyableObjectOverlayMat.M_DestroyableObjectOverlayMat" "None" "None" :!class /Script/Engine.KismetMaterialLibrary))
  (Rendering|Material|SetOverlayMaterial (Variables|Default|GetStaticMesh) _returnvalue :!class /Script/Engine.MeshComponent))

(event Collision|EventActorBeginOverlap
  (params (OtherActor :type Actor%20Object%20Reference)))

(event EventStopInteract
  (params (ActorStopingInteract :type Actor%20Object%20Reference))
  (bind _returnvalue (Game|GetPlayerController 0))
  (bind _asbp_myles (Utilities|Casting|CastToBP_Myles ActorStopingInteract))
  (Variables|/Game/MetaHumans/Myles/BP_Myles.BP_Myles_C|SetIsMovingFreely _asbp_myles true)
  (Collision|SetCollisionResponsetoChannel (Variables|Default|GetSphere) "ECC_GameTraceChannel1" "ECR_Block")
  (Input|SetInputModeGameOnly _returnvalue true)
  (Variables|/Script/Engine.PlayerController|SetbShowMouseCursor _returnvalue false)
  (Class|WidgetBlueprintLibrary|SetFocustoGameViewport)
  (Class|GameplayStatics|SetViewportMouseCaptureMode "CapturePermanently")
  (bind _asbp_myles_2 (Utilities|Casting|CastToBP_Myles (Game|Player|GetPlayerPawn 0)))
  (Default|SetSittingandTypingAnim _asbp_myles_2 false false)
  (Default|Writting _asbp_myles_2 false)
  (bind _asbp_base_paper (Utilities|Casting|CastToBP_BasePaper (Variables|/Script/Engine.ChildActorComponent|GetChildActor (Variables|Default|GetChildActor))))
  (Default|StopBasePaperWritting _asbp_base_paper))

(event EventTick
  (params (DeltaSeconds :type Float%20%28single-precision%29)))

(event EventOnHitbyPlayerLaser
  (bind _asmaterial_instance_dynamic (Utilities|Casting|CastToMaterialInstanceDynamic (Rendering|Material|GetOverlayMaterial (Variables|Default|GetStaticMesh) :!class /Script/Engine.MeshComponent)))
  (Rendering|Material|SetScalarParameterValue _asmaterial_instance_dynamic "HighlightStrenght" 1.0 :!class /Script/Engine.MaterialInstanceDynamic))

(event EventOnNoLongerHitbyPlayerLaser
  (bind _asmaterial_instance_dynamic (Utilities|Casting|CastToMaterialInstanceDynamic (Rendering|Material|GetOverlayMaterial (Variables|Default|GetStaticMesh) :!class /Script/Engine.MeshComponent)))
  (Rendering|Material|SetScalarParameterValue _asmaterial_instance_dynamic "HighlightStrenght" 0.0 :!class /Script/Engine.MaterialInstanceDynamic))

(fn ConstructionScript)

(fn ChangeGameModetoWriting
  (params (Object :type Object%20Object%20Reference) (self2 :type Player%20Controller%20Object%20Reference) (PlayerController :type Player%20Controller%20Object%20Reference))
  (bind _asbp_myles (Utilities|Casting|CastToBP_Myles Object))
  (Variables|/Game/MetaHumans/Myles/BP_Myles.BP_Myles_C|SetIsMovingFreely _asbp_myles false)
  (Collision|SetCollisionResponsetoChannel (Variables|Default|GetSphere) "ECC_GameTraceChannel1" "ECR_Ignore")
  (bind _asbp_base_paper (Utilities|Casting|CastToBP_BasePaper (Variables|/Script/Engine.ChildActorComponent|GetChildActor (Variables|Default|GetChildActor))))
  (Input|SetInputModeGameandUI PlayerController (Variables|/Game/WrittingPageMechanics/BP_BasePaper.BP_BasePaper_C|GetAs%20UW%20Base%20Paper _asbp_base_paper) "LockAlways" false false)
  (Variables|/Script/Engine.PlayerController|SetbShowMouseCursor self2 true))

(fn SpawnNewPaper
  (bind _returnvalue (AddComponent|AddChildActorComponent false (Variables|Default|GetChildActorRelativeTransform)))
  (Transformation|AttachComponentToComponent _returnvalue (Variables|Default|GetStaticMesh) "None" "KeepRelative" "KeepRelative" "KeepRelative" true))

(fn Interact
  (params (ActorThatInteract :type Actor%20Object%20Reference))
  (bind _returnvalue (Game|GetPlayerController 0))
  (bind _returnvalue_2 (Game|GetPlayerController 0))
  (CallFunction|ChangeGameModetoWriting ActorThatInteract _returnvalue_2 _returnvalue_2)
  (bind _asbp_myles (Utilities|Casting|CastToBP_Myles ActorThatInteract))
  (Pawn|UnPossess _returnvalue)
  (bind _returnvalue_3 (Game|SpawnActorfromClass "/Game/FirstPerson/Blueprints/BP_AIControllerPlayerPawn.BP_AIControllerPlayerPawn_C" (Transformation|GetActorTransform _asbp_myles) "Undefined" "MultiplyWithRoot" 0 (Transformation|GetWorldTransform (Variables|Default|GetStandingPlayerPosition)) 0))
  (bind _output_get (Variables|Default|SetNewVar_0 _returnvalue_3))
  (Pawn|Possess _output_get _asbp_myles)
  (Components|Activation|Activate (Variables|/Game/FirstPerson/Blueprints/BP_AGameAboutWrittingCharacter.BP_AGameAboutWrittingCharacter_C|GetFirstPersonCamera _asbp_myles) false)
  (Game|Player|SetViewTargetwithBlend _returnvalue ActorThatInteract 0.0 "VTBlend_Linear" 0.0 false)
  (return true))

(fn GetCancelActionName
  (return "Quit typing"))

(fn GetInteractionActionName
  (return "Start typing"))

(fn GetUseActionName
  (return ""))