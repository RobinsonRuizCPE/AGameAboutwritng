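; BP_BookInfo is an interactable book actor that opens on interaction and shows widget content on a screen material.
; BeginPlay sets the reference pose and creates dynamic overlay and screen materials; the player's laser hit events toggle the overlay highlight.
; Tick waits for the Widget's render target, then binds it once as the screen's emissive texture.
; Interact plays the opening animation, and StopInteract plays a montage in reverse from its end.
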(event EventBeginPlay
  (bind _staticmesh (Variables|Default|GetStaticMesh))
  (Components|Animation|PlayAnimation (Variables|Default|GetStaticMesh) "/Game/WrittingPageMechanics/Book/BBis/AP_BookRefPose.AP_BookRefPose" false)
  (bind _returnvalue (Rendering|Material|CreateDynamicMaterialInstance "/Game/FXMaterials/OverlayFx/M_DestroyableObjectOverlayMat.M_DestroyableObjectOverlayMat" "None" "None" :!class /Script/Engine.KismetMaterialLibrary))
  (Rendering|Material|SetOverlayMaterial (Variables|Default|GetStaticMesh) _returnvalue :!class /Script/Engine.MeshComponent)
  (bind _returnvalue_2 (Rendering|Material|CreateDynamicMaterialInstance _staticmesh 4 "/Game/Fab/TV_LCD/Screen.Screen" "None" :!class /Script/Engine.PrimitiveComponent))
  (bind _output_get (Variables|Default|SetScreenDynamicMaterial _returnvalue_2))
  (Rendering|Material|SetMaterial _staticmesh 4 _output_get))

(event Collision|EventActorBeginOverlap
  (params (OtherActor :type Actor%20Object%20Reference)))

(event EventTick
  (params (DeltaSeconds :type Float%20%28single-precision%29))
  (bind _widget (Variables|Default|GetWidget))
  (bind _returnvalue (Class|WidgetComponent|GetRenderTarget _widget))
  (if (not (Variables|Default|GetRenderTargetIsSet))
    (Utilities|IsValid _returnvalue
      (:Is%20Valid
        (Rendering|Material|SetTextureParameterValue (Variables|Default|GetScreenDynamicMaterial) "EmissiveTexture" _returnvalue)
        (Variables|Default|SetRenderTargetIsSet true)))))

(event EventStopInteract
  (params (ActorStopingInteract :type Actor%20Object%20Reference))
  (bind _montage_to_play (Variables|Default|GetMontage%20to%20Play))
  (Animation|Montage|PlayMontage (Variables|Default|GetStaticMesh) _montage_to_play -1.0 (Animation|GetPlayLength _montage_to_play)))

(event EventOnHitbyPlayerLaser
  (bind _asmaterial_instance_dynamic (Utilities|Casting|CastToMaterialInstanceDynamic (Rendering|Material|GetOverlayMaterial (Variables|Default|GetStaticMesh) :!class /Script/Engine.MeshComponent)))
  (Rendering|Material|SetScalarParameterValue _asmaterial_instance_dynamic "HighlightStrenght" 1.0 :!class /Script/Engine.MaterialInstanceDynamic))

(event EventOnNoLongerHitbyPlayerLaser
  (bind _asmaterial_instance_dynamic (Utilities|Casting|CastToMaterialInstanceDynamic (Rendering|Material|GetOverlayMaterial (Variables|Default|GetStaticMesh) :!class /Script/Engine.MeshComponent)))
  (Rendering|Material|SetScalarParameterValue _asmaterial_instance_dynamic "HighlightStrenght" 0.0 :!class /Script/Engine.MaterialInstanceDynamic))

(fn ConstructionScript)

(fn Interact
  (params (ActorThatInteract :type Actor%20Object%20Reference))
  (Components|Animation|PlayAnimation (Variables|Default|GetStaticMesh) "/Game/WrittingPageMechanics/Book/BBis/NewBookRefPoseOpenBookAction.NewBookRefPoseOpenBookAction" false)
  (return true))