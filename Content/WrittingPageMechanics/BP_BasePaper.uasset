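; BP_BasePaper is a typewriter page actor hosting a UW_BasePaper text widget that the player types on.
; Line-count changes shift the page vertically by scaled line height.
; A full page locks input, rings a bell and shows UW_RatingPaper to score the text.
; When the review wraps up, the page detaches, glides to its reviewed position via timeline, then tells parent BP_Typewritter to spawn new paper.
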(event Custom|OnFinishedWrappingUp
  (bind _widget (Variables|Default|GetWidget))
  (Widget|RemovefromParent (Variables|Default|GetRatingPaper))
  (Transformation|DetachFromActor "KeepWorld" "KeepWorld" "KeepWorld")
  (Variables|Default|SetPageCompletePos (Transformation|GetWorldTransform (Variables|Default|GetPageReviewedTransform)))
  (Components|Timeline|SetPlayRate (Variables|Default|GetTimeline) (/ 1.0 (Variables|Default|GetPageMovementRate)))
  (bind _timeelapsed (Timeline|Timeline PlayFromStart)
    (:Update
      (Transformation|SetActorTransform (Math|Transform|Lerp(Transform) (Transformation|GetWorldTransform (Variables|Default|GetScene)) (Variables|Default|GetPageCompletePos) _timeelapsed)))
    (:Finished
      (bind _asbp_typewritter (Utilities|Casting|CastToBP_Typewritter (Actor|GetParentActor)))
      (Default|SpawnNewPaper _asbp_typewritter)
      (Class|WidgetComponent|SetWindowFocusable _widget false)
      (Class|WidgetComponent|SetWindowVisibility _widget "SelfHitTestInvisible")
      (EventDispatchers|UnbindEventfromOnFinishedWrapUp (Variables|Default|GetRatingPaper) (delegate Custom|OnFinishedWrappingUp)))))

(event Custom|CustomEvent
  (params (NewLineCount :type Integer) (PreviousLineCount :type Integer) (LineHeight :type Float%20%28single-precision%29))
  (Utilities|HandleNewLineMovement NewLineCount PreviousLineCount LineHeight))

(event Custom|OnPage%20filled
  (params (TextToAnalyse :type Text))
  (Utilities|FlowControl|Delay 0.1)
  (if (not (Variables|Default|GetReviewInProgress))
    (Variables|Default|SetReviewInProgress true)
    (Utilities|HandlePageFilled TextToAnalyse)))

(event EventBeginPlay
  (Variables|Default|SetSpawn%20Transform (Transformation|GetWorldTransform (Variables|Default|GetScene)))
  (bind _returnvalue (UserInterface|CreateWidget "/Game/WrittingPageMechanics/UW_RatingPaper.UW_RatingPaper_C"))
  (Variables|Default|SetRatingPaper _returnvalue)
  (bind _asuw_base_paper (Utilities|Casting|CastToUW_BasePaper (UserInterface|GetUserWidgetObject (Variables|Default|GetWidget))))
  (bind _output_get (Variables|Default|SetAs%20UW%20Base%20Paper _asuw_base_paper))
  (Utilities|CopyFontforReviewPaper _output_get)
  (EventDispatchers|BindEventtoOnLineCountChanged (Variables|Default|GetAs%20UW%20Base%20Paper) (delegate Custom|CustomEvent))
  (EventDispatchers|BindEventtoOnPageFull (Variables|Default|GetAs%20UW%20Base%20Paper) (delegate Custom|OnPage%20filled))
  (EventDispatchers|BindEventtoOnFinishedWrapUp (Variables|Default|GetRatingPaper) (delegate Custom|OnFinishedWrappingUp)))

(event Collision|EventActorBeginOverlap
  (params (OtherActor :type Actor%20Object%20Reference)))

(event EventTick
  (params (DeltaSeconds :type Float%20%28single-precision%29)))

(fn ConstructionScript)

(fn StopBasePaperWritting
  (Default|StopTypingSound (Variables|Default|GetAs%20UW%20Base%20Paper)))