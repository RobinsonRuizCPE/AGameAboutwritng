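; Interactable actor that shows the total-stats widget on screen when the player interacts with it.
; BeginPlay puts a dynamic overlay material on its static mesh, and player laser hit events toggle that material's highlight strength on and off.
; Interact creates UW_TotalStatsDispalyer for the first player and adds it to the viewport; StopInteract removes it.
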(event EventBeginPlay
  (bind _returnvalue (Rendering|Material|CreateDynamicMaterialInstance "/Game/FXMaterials/OverlayFx/M_DestroyableObjectOverlayMat.M_DestroyableObjectOverlayMat" "None" "None" :!class /Script/Engine.KismetMaterialLibrary))
  (Rendering|Material|SetOverlayMaterial (Variables|Default|GetStaticMesh) _returnvalue :!class /Script/Engine.MeshComponent))

(event Collision|EventActorBeginOverlap
  (params (OtherActor :type Actor%20Object%20Reference)))

(event EventTick
  (params (DeltaSeconds :type Float%20%28single-precision%29)))

(event EventOnHitbyPlayerLaser
  (bind _asmaterial_instance_dynamic (Utilities|Casting|CastToMaterialInstanceDynamic (Rendering|Material|GetOverlayMaterial (Variables|Default|GetStaticMesh) :!class /Script/Engine.MeshComponent)))
  (Rendering|Material|SetScalarParameterValue _asmaterial_instance_dynamic "HighlightStrenght" 1.0 :!class /Script/Engine.MaterialInstanceDynamic))

(event EventOnNoLongerHitbyPlayerLaser
  (bind _asmaterial_instance_dynamic (Utilities|Casting|CastToMaterialInstanceDynamic (Rendering|Material|GetOverlayMaterial (Variables|Default|GetStaticMesh) :!class /Script/Engine.MeshComponent)))
  (Rendering|Material|SetScalarParameterValue _asmaterial_instance_dynamic "HighlightStrenght" 0.0 :!class /Script/Engine.MaterialInstanceDynamic))

(event EventStopInteract
  (params (ActorStopingInteract :type Actor%20Object%20Reference))
  (Widget|RemovefromParent (Variables|Default|GetWidget)))

(fn ConstructionScript)

(fn Interact
  (params (ActorThatInteract :type Actor%20Object%20Reference))
  (bind _returnvalue (UserInterface|CreateWidget "/Game/UI/EndOfGameUI/UW_TotalStatsDispalyer.UW_TotalStatsDispalyer_C" (Game|GetPlayerController 0)))
  (bind _output_get (Variables|Default|SetWidget _returnvalue))
  (UserInterface|Viewport|AddtoViewport _output_get 10)
  (return false))